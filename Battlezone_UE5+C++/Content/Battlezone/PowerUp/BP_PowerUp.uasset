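; BP_PowerUp is a pickup that notifies an overlapping BP_TankPlayer through PickedPowerUp, then relocates once consumed.
; BeginPlay caches all TargetPoints tagged "Tpower" as candidate spawn locations.
; ConsumePickable deactivates and hides it, waits briefly (one second, despite a comment saying 15), then teleports it to a random cached point.
; It retries until SetActorLocation succeeds, then becomes active and visible again.
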(event `self.ReceiveBeginPlay`
  ;[1 1 1] Initialise the array of TargetPoints
  (bind _outactors (`GameplayStatics.GetAllActorsOfClassWithTag` "/Script/Engine.TargetPoint" "Tpower"))
  (set `self.TargetPointsArray` _outactors))

(event `self.Box.OnComponentBeginOverlap`
  (params (OverlappedComponent :type "PrimitiveComponent Object Reference") (OtherActor :type "Actor Object Reference") (OtherComp :type "PrimitiveComponent Object Reference") (OtherBodyIndex :type Integer) (bFromSweep :type Boolean) (SweepResult :type "HitResult Structure (by ref)"))
  ;[1 1 1] Player pick up power up
  (if (`self.bActive`)
    (bind _asbp_tank_player (cast `/Game/Battlezone/Tank/BP_TankPlayer` OtherActor))
    (`/Engine/EditorBlueprintResources/StandardMacros.IsValid` _asbp_tank_player
      (:`Is Valid`
        (`/Game/Battlezone/Tank/BP_TankPlayer.PickedPowerUp` _asbp_tank_player self)))))

(event `ConsumePickable`
  ;[1 1 1] Pickup consumed, unsuable and invisible for 15 sec before re-appearing
  (bind _output_get (set `self.bActive` false))
  (`SceneComponent.SetVisibility` (`self.Cube`) _output_get false)
  (`KismetSystemLibrary.Delay` 1.0)
  (bind (_sweephitresult _returnvalue) (`self.K2_SetActorLocation` (`self.K2_GetActorLocation` (`KismetArrayLibrary.Array_Random` (`self.TargetPointsArray`))) false true :!label _label))
  (if _returnvalue
    (bind _output_get_2 (set `self.bActive` true))
    (`SceneComponent.SetVisibility` (`self.Cube`) _output_get_2 false)
    (else
      (goto _label))))

(fn `UserConstructionScript`)