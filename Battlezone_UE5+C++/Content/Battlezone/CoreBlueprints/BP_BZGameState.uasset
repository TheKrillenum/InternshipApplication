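; Game State for a Battlezone tank match, handling tank spawning, possession, scoring, lives and the current leader.
; Tick switches on StateSwitch with DoOnce gates, spawning four tanks at tagged target points during preparation, then enabling input and clearing player loading when play starts.
; PlayerDestroyed awards kill points, then respawns the victim in a new tank at a random point or unpossesses when lives run out.
; A self-recalling one-second loop tracks the top scorer.
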(event `PossessTanks`
  (`self.PlayerPossessTank`))

(event `self.ReceiveTick`
  (params (DeltaSeconds :type "Float (single-precision)"))
  (switch `/Game/Battlezone/CoreBlueprints/EGameState` (`self.StateSwitch`)
    (:`NewEnumerator2`
      (`/Engine/EditorBlueprintResources/StandardMacros.DoOnce` false
        (:`Completed`
          (`self.SpawnTanks`))))
    (:`NewEnumerator3`
      (`/Engine/EditorBlueprintResources/StandardMacros.DoOnce` false
        (:`Completed`
          (bind _outactors (`GameplayStatics.GetAllActorsOfClass` "/Game/Battlezone/Tank/BP_TankPlayer.BP_TankPlayer_C"))
          (for _array_element _outactors
            (`self.DisableInput` _array_element null))
          (for _array_element_2 (`self.PlayerArray`)
            (`KismetArrayLibrary.Array_AddUnique` (`self.NameArray`) (`PlayerState.GetPlayerName` _array_element_2)))
          (bind _outactors_2 (`GameplayStatics.GetAllActorsOfClass` "/Game/Battlezone/Tank/BP_TankPlayer.BP_TankPlayer_C"))
          (for _array_element_3 _outactors_2
            (`/Game/Battlezone/Tank/BP_TankPlayer.ActivateInput` _array_element_3))
          (for _array_element_4 (`self.PlayerArray`)
            (bind _asbp_bzplayer_state (cast `/Game/Battlezone/CoreBlueprints/BP_BZPlayerState` _array_element_4))
            (`/Engine/EditorBlueprintResources/StandardMacros.IsValid` _asbp_bzplayer_state
              (:`Is Valid`
                (`/Game/Battlezone/CoreBlueprints/BP_BZPlayerState.LoadingOver` _asbp_bzplayer_state)))))))))

(event `self.ReceiveBeginPlay`
  ;[1 1 1] Initialize Game Mode
  (bind _asbp_bzgame_mode (cast `/Game/Battlezone/CoreBlueprints/BP_BZGameMode` (`GameplayStatics.GetGameMode`)))
  (`/Engine/EditorBlueprintResources/StandardMacros.IsValid` _asbp_bzgame_mode
    (:`Is Valid`
      (set `self.RefGameMode` _asbp_bzgame_mode)
      (`self.BestPoints&Player`))))

(event `PlayerDestroyed`
  (params (ScoringPlayer :type "/Game/Battlezone/CoreBlueprints/BP_BZPlayerState Object Reference") (DestroyedPlayer :type "/Game/Battlezone/CoreBlueprints/BP_BZPlayerState Object Reference"))
  (bind _returnvalue (`PlayerState.GetPlayerController` DestroyedPlayer))
  ;[1 1 1] Logic for when a player kills another
  (`|ExecutionSequence`
    (:`then_0`
      ;;[1 1 1] Award points to the player who got the kill
      (bind _output_get (set `/Game/Battlezone/CoreBlueprints/BP_BZPlayerState.PlayerScore` (+ (`/Game/Battlezone/CoreBlueprints/BP_BZPlayerState.PlayerScore` ScoringPlayer) 500) ScoringPlayer))
      (if (or (== _output_get 1000) (== _output_get 2000))
        (`/Engine/EditorBlueprintResources/StandardMacros.IncrementInt` (`/Game/Battlezone/CoreBlueprints/BP_BZPlayerState.PlayerLives` ScoringPlayer)
          (:`  `
            (set `/Game/Battlezone/CoreBlueprints/BP_BZPlayerState.PlayerLives` 0 ScoringPlayer)))))
    (:`then_1`
      ;;[1 1 1] Reduce life count, unpossess the "destroyed" tank and possess a new one
      (bind _result (`/Engine/EditorBlueprintResources/StandardMacros.DecrementInt` (`/Game/Battlezone/CoreBlueprints/BP_BZPlayerState.PlayerLives` DestroyedPlayer))
        (:`  `
          (if (<= _result 0)
            ;;[1 1 1] Go back to spectator mode if there is no life left
            (`Controller.UnPossess` (`PlayerState.GetPlayerController` DestroyedPlayer))
            (else
              (bind _returnvalue_2 (`|SpawnActorFromClass` "/Game/Battlezone/Tank/BP_TankPlayer.BP_TankPlayer_C" (`self.GetTransform` (`KismetArrayLibrary.Array_Random` (`self.TargetPoints`))) "AdjustIfPossibleButAlwaysSpawn" "MultiplyWithRoot" null null))
              (`Controller.UnPossess` _returnvalue)
              (`Controller.Possess` _returnvalue _returnvalue_2))))))))

(event `BestPoints&Player`
  (for _array_element (`self.PlayerArray`)
    (bind _asbp_bzplayer_state (cast `/Game/Battlezone/CoreBlueprints/BP_BZPlayerState` _array_element))
    (`/Engine/EditorBlueprintResources/StandardMacros.IsValid` _asbp_bzplayer_state
      (:`Is Valid`
        (bind _playerscore (`/Game/Battlezone/CoreBlueprints/BP_BZPlayerState.PlayerScore` _asbp_bzplayer_state))
        (if (> _playerscore (`self.BestPoint`))
          (set `self.BestPoint` _playerscore)
          (set `self.BestPlayer` (`PlayerState.GetPlayerName` _asbp_bzplayer_state))))))
  (`KismetSystemLibrary.Delay` 1.0)
  (`self.BestPoints&Player`))

(fn `OnRep_StateSwitch`)

(fn `PlayerPossessTank`
  (for (_array_element _array_index) (`self.PlayerArray`)
    (`Controller.Possess` (`PlayerState.GetPlayerController` _array_element) (`|GetArrayItem` (`self.Tanks`) _array_index))))

(fn `SpawnTanks`
  (bind _outactors (`GameplayStatics.GetAllActorsOfClassWithTag` "/Script/Engine.TargetPoint" "Tspawn"))
  (set `self.TargetPoints` _outactors)
  (for _index (range 4)
    (bind _returnvalue (`|SpawnActorFromClass` "/Game/Battlezone/Tank/BP_TankPlayer.BP_TankPlayer_C" (`self.GetTransform` (`|GetArrayItem` (`self.TargetPoints`) _index)) "AdjustIfPossibleButAlwaysSpawn" "MultiplyWithRoot" null null))
    (`KismetArrayLibrary.Array_Add` (`self.Tanks`) _returnvalue))
  (return))

(fn `UserConstructionScript`
  (set `self.bTankReady` false))