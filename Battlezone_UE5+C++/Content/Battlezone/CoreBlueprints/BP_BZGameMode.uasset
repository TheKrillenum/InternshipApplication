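; Battlezone game mode that manages player joins and game state across menu, lobby and match levels.
; BeginPlay caches the game instance and state, derives the state from the level name, and flushes players queued by early logins.
; Lobby joins register in the GameState's player array and possess temporary first-person characters.
; Match levels use fixed delays before possessing tanks and advancing state; match travel goes through the game instance.
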(event `SwitchStates`
  (params (NewParam :type "/Game/Battlezone/CoreBlueprints/EGameState Enum" :default "NewEnumerator1"))
  ;[1 1 1] Outside call to change the state of the game
  (set `/Game/Battlezone/CoreBlueprints/BP_BZGameState.StateSwitch` NewParam (`self.RefGameState`)))

(event `self.ReceiveBeginPlay`
  ;[1 1 1] Begin play, initialise variables
  (bind _asbzgame_instance (cast `BZGameInstance` (`GameplayStatics.GetGameInstance`)))
  (`/Engine/EditorBlueprintResources/StandardMacros.IsValid` _asbzgame_instance
    (:`Is Valid`
      (set `self.RefGameInstance` _asbzgame_instance)
      (bind _asbp_bzgame_state (cast `/Game/Battlezone/CoreBlueprints/BP_BZGameState` (`GameplayStatics.GetGameState`)))
      (`/Engine/EditorBlueprintResources/StandardMacros.IsValid` _asbp_bzgame_state
        (:`Is Valid`
          (bind _output_get (set `self.RefGameState` _asbp_bzgame_state))
          (`/Engine/EditorBlueprintResources/StandardMacros.IsValid` _output_get
            (:`Is Valid`
              (bind _game_state (`self.SetGameStateSwitch` _output_get))
              (`self.EmptyWaitingQueue`)
              (if (== _game_state 2)
                ;[1 1 1] A bit of cheating :P
                (`KismetSystemLibrary.Delay` 8.0)
                (`/Game/Battlezone/CoreBlueprints/BP_BZGameState.PossessTanks` (`self.RefGameState`))
                (`KismetSystemLibrary.Delay` 2.0)
                (`self.SwitchStates` "NewEnumerator3")))))))))

(event `TravelToMatch`
  ;[1 1 1] Travel to the map where the match unfolds
  (`BZGameInstance.StartLevel` (`self.RefGameInstance`)))

(event `self.K2_PostLogin`
  (params (NewPlayer :type "PlayerController Object Reference"))
  ;[1 1 1] Players joining logic
  ;;[1 1 1] Player joined: add them to waiting queue if GameState is not ready, otherwise take care of them
  (`KismetSystemLibrary.PrintString` "sheesh")
  (if (`KismetSystemLibrary.IsValid` (`self.RefGameState`))
    (`self.AddToPlayerList` (`Controller.PlayerState` NewPlayer))
    (else
      (`self.PlayerWaitingQueue` NewPlayer))))

(event `PlayerWaitingQueue`
  (params (`Player Controller` :type "PlayerController Object Reference"))
  ;[1 1 1] Players joining logic
  ;;[1 1 1] Add player that arrived before "begin play" to a waiting queue"
  (`KismetArrayLibrary.Array_Add` (`self.WaitingList`) `Player Controller`))

(event `EmptyWaitingQueue`
  (bind _waitinglist (`self.WaitingList`))
  ;[1 1 1] Players joining logic
  ;;[1 1 1] Allow all players in the waiting to queue to try and join the player list again
  (if (`KismetArrayLibrary.Array_IsNotEmpty` _waitinglist)
    (for _array_element _waitinglist
      (`self.AddToPlayerList` (`Controller.PlayerState` _array_element)))
    (`KismetArrayLibrary.Array_Clear` _waitinglist)))

(event `AddToPlayerList`
  (params (NewPlayerState :type "PlayerState Object Reference"))
  (bind _refgamestate (`self.RefGameState`))
  (bind _playerarray (`GameStateBase.PlayerArray` _refgamestate))
  (bind _playerarray_2 (`GameStateBase.PlayerArray` (`self.RefGameState`)))
  ;[1 1 1] Players joining logic
  ;;[1 1 1] Check if the given player isn't already in the array of players
  (if (`|EnumEquality` (`/Game/Battlezone/CoreBlueprints/BP_BZGameState.StateSwitch` _refgamestate) "NewEnumerator0")
    (bind _asbp_bzplayer_state (cast `/Game/Battlezone/CoreBlueprints/BP_BZPlayerState` NewPlayerState))
    (`/Engine/EditorBlueprintResources/StandardMacros.IsValid` _asbp_bzplayer_state
      (:`Is Valid`
        (if (`KismetArrayLibrary.Array_Contains` _playerarray _asbp_bzplayer_state)
          ;;[1 1 1] Replace the player in the player array if he already exist
          (`KismetArrayLibrary.Array_Set` _playerarray_2 (`KismetArrayLibrary.Array_Find` _playerarray_2 _asbp_bzplayer_state) _asbp_bzplayer_state)
          (else
            ;;[1 1 1] Add the new player to the array of players
            (`KismetArrayLibrary.Array_Add` _playerarray _asbp_bzplayer_state)))
        ;;[1 1 1] If we are currently in the lobby map, player possess a temporary first player character body
        (bind _returnvalue (`GameplayStatics.GetActorOfClass` "/Script/Engine.PlayerStart"))
        (bind _returnvalue_2 (`|SpawnActorFromClass` "/Game/FirstPerson/Blueprints/BP_FirstPersonCharacter.BP_FirstPersonCharacter_C" (`self.GetTransform` _returnvalue) "Undefined" "MultiplyWithRoot" null null))
        (`Controller.Possess` (`PlayerState.GetPlayerController` _asbp_bzplayer_state) _returnvalue_2)))))

(fn `SetGameStateSwitch`
  (params (GameState :type "/Game/Battlezone/CoreBlueprints/BP_BZGameState Object Reference"))
  (returns (`Game state` :type "/Game/Battlezone/CoreBlueprints/EGameState Enum"))
  (bind _returnvalue (`GameplayStatics.GetCurrentLevelName` true))
  (if (`KismetStringLibrary.EqualEqual_StrStr` _returnvalue "MainMenuLevel")
    (set `/Game/Battlezone/CoreBlueprints/BP_BZGameState.StateSwitch` "NewEnumerator1" GameState)
    (else
      (bind _returnvalue_2 (`GameplayStatics.GetCurrentLevelName` true))
      (if (`KismetStringLibrary.EqualEqual_StrStr` _returnvalue_2 "Lobby")
        (set `/Game/Battlezone/CoreBlueprints/BP_BZGameState.StateSwitch` "NewEnumerator0" GameState)
        (else
          (set `/Game/Battlezone/CoreBlueprints/BP_BZGameState.StateSwitch` "NewEnumerator2" GameState)))))
  (return (`/Game/Battlezone/CoreBlueprints/BP_BZGameState.StateSwitch` GameState)))

(fn `UserConstructionScript`)