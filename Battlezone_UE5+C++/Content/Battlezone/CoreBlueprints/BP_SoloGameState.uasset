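; Solo-mode game state for Battlezone that runs tank spawning, respawns and kill scoring.
; BeginPlay gathers "Tspawn" target points, spawns the initial AI tanks and possesses the placed player tank.
; Kill events increment player score or decrease lives, then respawn a tank at a random point after a delay.
; GetTargetPoint refetches all points whenever the list is non-empty, undoing earlier removals of used points.
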(event `SpawnAI`
  ;[1 1 1] Spawning AI
  (bind _target_point (`self.GetTargetPoint`))
  (`|SpawnActorFromClass` "/Game/Battlezone/Tank/BP_TankAI.BP_TankAI_C" (`self.GetTransform` _target_point) "AdjustIfPossibleButAlwaysSpawn" "MultiplyWithRoot" null null)
  (`KismetArrayLibrary.Array_RemoveItem` (`self.TargetPoints`) _target_point))

(event `self.ReceiveBeginPlay`
  ;[1 1 1] Begin play, spawn all actors
  (`|ExecutionSequence`
    (:`then_0`
      (bind _outactors (`GameplayStatics.GetAllActorsOfClassWithTag` "/Script/Engine.TargetPoint" "Tspawn"))
      (set `self.TargetPoints` _outactors))
    (:`then_1`
      (for _ (range 3)
        (`self.SpawnAI`)))
    (:`then_2`
      (bind _returnvalue (`GameplayStatics.GetActorOfClass` "/Game/Battlezone/Tank/BP_TankPlayer.BP_TankPlayer_C"))
      (`Controller.Possess` (`GameplayStatics.GetPlayerController` 0) _returnvalue))))

(event `BotKilled`
  (params (Perpetrator :type "Actor Object Reference"))
  ;[1 1 1] Bot killed, award points
  (bind _asbp_tank_player (cast `/Game/Battlezone/Tank/BP_TankPlayer` Perpetrator)
    (:`then`
      (`/Engine/EditorBlueprintResources/StandardMacros.IsValid` _asbp_tank_player
        (:`Is Valid`
          (bind _asbp_bzplayer_state (cast `/Game/Battlezone/CoreBlueprints/BP_BZPlayerState` (`Pawn.PlayerState` _asbp_tank_player))
            (:`then`
              (`/Game/Battlezone/CoreBlueprints/BP_BZPlayerState.IncrementScore` _asbp_bzplayer_state))
            (:`CastFailed`
              _)))
        (:`Is Not Valid`
          _)))
    (:`CastFailed`
      _))
  ;[1 1 1] Respawn another bot
  (`KismetSystemLibrary.Delay` 2.0)
  (`self.SpawnAI`))

(event `PlayerKilled`
  (params (Player :type "/Game/Battlezone/CoreBlueprints/BP_BZPlayerState Object Reference"))
  ;[1 1 1] Decrease player HP. and respawn another tank to posses
  (`/Game/Battlezone/CoreBlueprints/BP_BZPlayerState.DecreaseLives` Player)
  (`KismetSystemLibrary.Delay` 2.75)
  (bind _target_point (`self.GetTargetPoint`))
  (bind _returnvalue (`|SpawnActorFromClass` "/Game/Battlezone/Tank/BP_TankPlayer.BP_TankPlayer_C" (`self.GetTransform` _target_point) "AdjustIfPossibleButAlwaysSpawn" "MultiplyWithRoot" null null))
  (`KismetArrayLibrary.Array_RemoveItem` (`self.TargetPoints`) _target_point)
  (`Controller.Possess` (`PlayerState.GetPlayerController` Player) _returnvalue))

(event `PointsUpdate`
  (params (`Player points` :type Integer))
  (set `self.PlayerPoints` `Player points`))

(fn `GetTargetPoint`
  (returns (`Target Point` :type "TargetPoint Object Reference"))
  (if (not (`KismetArrayLibrary.Array_IsEmpty` (`self.TargetPoints`)))
    (bind _outactors (`GameplayStatics.GetAllActorsOfClassWithTag` "/Script/Engine.TargetPoint" "Tspawn"))
    (set `self.TargetPoints` _outactors))
  (return (`KismetArrayLibrary.Array_Random` (`self.TargetPoints`))))

(fn `UserConstructionScript`)