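; Player state for the Battlezone tank game that tracks score and lives and owns the player's tank HUD.
; Outside the lobby and main menu, BeginPlay creates the HUD and caches either the standard or solo game state.
; Events push score, lives, power, enemy distance and active-screen changes to the widget.
; Fixed score increments award a bonus life every 10,000 points and, in SoloLevel, report the total to the solo game state.
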(event `self.ReceiveBeginPlay`
  (bind _returnvalue (`GameplayStatics.GetGameState`))
  ;[1 1 1] Initialise tank HUD
  (bind _returnvalue_2 (`GameplayStatics.GetCurrentLevelName` true))
  (if (and (`KismetStringLibrary.NotEqual_StrStr` _returnvalue_2 "Lobby") (`KismetStringLibrary.NotEqual_StrStr` _returnvalue_2 "MainMenuLevel"))
    (bind _returnvalue_3 (`|CreateWidget` "/Game/Battlezone/UI/IngameUI/WBP_TankInterface.WBP_TankInterface_C"))
    (bind _output_get (set `self.PlayerUI` _returnvalue_3))
    (`UserWidget.AddToViewport` _output_get 0)
    ;[1 1 1] Init ref Game state
    (bind _asbp_bzgame_state (cast `/Game/Battlezone/CoreBlueprints/BP_BZGameState` _returnvalue)
      (:`then`
        (`/Engine/EditorBlueprintResources/StandardMacros.IsValid` _asbp_bzgame_state
          (:`Is Valid`
            (set `self.RefGameState` _asbp_bzgame_state))
          (:`Is Not Valid`
            (bind _asbp_solo_game_state (cast `/Game/Battlezone/CoreBlueprints/BP_SoloGameState` _returnvalue :!label _label))
            (`/Engine/EditorBlueprintResources/StandardMacros.IsValid` _asbp_solo_game_state
              (:`Is Valid`
                (set `self.RefSoloGameState` _asbp_solo_game_state))))))
      (:`CastFailed`
        (goto _label)))))

(event `IndexUI`
  (params (NewParam :type Integer))
  ;[1 1 1] Change the active widget of the UI
  (set `WidgetSwitcher.ActiveWidgetIndex` NewParam (`/Game/Battlezone/UI/IngameUI/WBP_TankInterface.WidgetSwitcher_73` (`self.PlayerUI`))))

(event `IncrementScore`
  ;[1 1 1] Increment player score
  (bind _output_get (set `self.PlayerScore` (+ (`self.PlayerScore`) 500)))
  (`/Game/Battlezone/UI/IngameUI/WBP_TankInterface.UpdateScore` (`self.PlayerUI`) _output_get)
  ;[1 1 1] Check if the player gets bonus HP based on his score (10k)
  (bind _output_get_2 (set `self.BonusLifeCounter` (+ (`self.BonusLifeCounter`) 500)))
  (if (>= _output_get_2 10000)
    (set `self.BonusLifeCounter` 0)
    (`self.BonusHP`)
    (bind _returnvalue (`GameplayStatics.GetCurrentLevelName` true)))
  (if (`KismetStringLibrary.EqualEqual_StrStr` _returnvalue "SoloLevel")
    (`/Game/Battlezone/CoreBlueprints/BP_SoloGameState.PointsUpdate` (`self.RefSoloGameState`) _output_get)))

(event `DecreaseLives`
  ;[1 1 1] Decrement player lives
  (bind _result (`/Engine/EditorBlueprintResources/StandardMacros.DecrementInt` (`self.PlayerLives`))
    (:`  `
      (`/Game/Battlezone/UI/IngameUI/WBP_TankInterface.UpdateLives` (`self.PlayerUI`) _result))))

(event `BonusHP`
  ;[1 1 1] Give player bonus life
  (bind _result (`/Engine/EditorBlueprintResources/StandardMacros.IncrementInt` (`self.PlayerLives`))
    (:`  `
      (`/Game/Battlezone/UI/IngameUI/WBP_TankInterface.UpdateLives` (`self.PlayerUI`) _result))))

(event `HasPower`
  (params (bHasPower :type Boolean))
  ;[1 1 1] Power on/off
  (`/Game/Battlezone/UI/IngameUI/WBP_TankInterface.UpdatePower` (`self.PlayerUI`) bHasPower))

(event `Distance to enemy`
  (params (Distance :type "Float (double-precision)"))
  ;[1 1 1] Display distance to enemy
  (`/Game/Battlezone/UI/IngameUI/WBP_TankInterface.DistanceDisplay` (`self.PlayerUI`) Distance))

(event `LoadingOver`
  ;[1 1 1] Loading over
  (`WidgetSwitcher.SetActiveWidgetIndex` (`/Game/Battlezone/UI/IngameUI/WBP_TankInterface.WidgetSwitcher_73` (`self.PlayerUI`)) 1))

(fn `UserConstructionScript`)