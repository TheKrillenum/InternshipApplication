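; Player tank pawn for Battlezone, serving both solo and PVP modes.
; Enhanced Input drives movement, yaw look, rate-limited projectile fire and pausing; multiplayer disables input on possession, with ActivateInput to enable it.
; An enemy projectile hit consumes the power-up shield or kills the tank, reporting to the PVP or solo game state.
; Each tick, a forward line trace sends the distance to a tank ahead to the player state.
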(event `self.ReceiveBeginPlay`
  (bind _returnvalue (`GameplayStatics.GetGameState`))
  ;[1 1 1] Initialise game state ref
  (bind _asbp_bzgame_state (cast `/Game/Battlezone/CoreBlueprints/BP_BZGameState` _returnvalue)
    (:`then`
      (`/Engine/EditorBlueprintResources/StandardMacros.IsValid` _asbp_bzgame_state
        (:`Is Valid`
          (set `self.PVPGameState` _asbp_bzgame_state))))
    (:`CastFailed`
      ;[1 1 1] Ref game state (in solo game)
      (bind _asbp_solo_game_state (cast `/Game/Battlezone/CoreBlueprints/BP_SoloGameState` _returnvalue))
      (`/Engine/EditorBlueprintResources/StandardMacros.IsValid` _asbp_solo_game_state
        (:`Is Valid`
          (set `self.RefPVEGameState` _asbp_solo_game_state)))))
  ;[1 1 1] Initialise Game instant ref
  (bind _asbzgame_instance (cast `BZGameInstance` (`GameplayStatics.GetGameInstance`)))
  (`/Engine/EditorBlueprintResources/StandardMacros.IsValid` _asbzgame_instance
    (:`Is Valid`
      (set `self.RefGameInst` _asbzgame_instance)
      ;[1 1 1] Starting values
      (set `self.bHasPower` false)
      (set `self.bCanShoot` true)
      (set `self.bAlive` true))))

(event `TankDisabled`
  (bind _returnvalue (`self.GetOwner`))
  ;[1 1 1] Disable input
  (if (`self.bAI`)
    (bind _asbp_bzaicontroller (cast `/Game/Battlezone/Tank/TankAI/BP_BZAIController` _returnvalue))
    (`self.DisableInput` _asbp_bzaicontroller null)
    (else
      (bind _asbp_first_person_player_controller (cast `/Game/FirstPerson/Blueprints/BP_FirstPersonPlayerController` _returnvalue))
      (`self.DisableInput` _asbp_first_person_player_controller))))

(event `self.ReceivePossessed`
  (params (NewController :type "Controller Object Reference"))
  ;[1 1 1] Disable input if it's a multiplayer game
  (bind _returnvalue (`GameplayStatics.GetCurrentLevelName` true))
  (if (`KismetStringLibrary.EqualEqual_StrStr` _returnvalue "SoloLevel")
    ;[1 1 1] PauseMenuRef
    (bind _returnvalue_2 (`BZGameInstance.LoadPauseMenu` (`self.RefGameInst`)))
    (`/Engine/EditorBlueprintResources/StandardMacros.IsValid` _returnvalue_2
      (:`Is Valid`
        (bind _output_get (set `self.RefPauseWidget` _returnvalue_2))
        (`Widget.SetVisibility` _output_get "Hidden")
        ;[1 1 1] Init ref player state
        (bind _asbp_bzplayer_state (cast `/Game/Battlezone/CoreBlueprints/BP_BZPlayerState` (`self.PlayerState`)))
        (`/Engine/EditorBlueprintResources/StandardMacros.IsValid` _asbp_bzplayer_state
          (:`Is Valid`
            (set `self.RefPlayerState` _asbp_bzplayer_state)))))
    (else
      (bind _asbp_first_person_player_controller (cast `/Game/FirstPerson/Blueprints/BP_FirstPersonPlayerController` NewController))
      (`/Engine/EditorBlueprintResources/StandardMacros.IsValid` _asbp_first_person_player_controller
        (:`Is Valid`
          (`self.DisableInput` _asbp_first_person_player_controller))))))

(event `Shooting`
  (bind (_returnvalue_location _returnvalue_rotation) (`KismetMathLibrary.BreakTransform` (`SceneComponent.K2_GetComponentToWorld` (`self.ProjectileSpawn`))))
  ;[1 1 1] Shooting
  (`|SpawnActorFromClass` "/Game/Battlezone/Tank/Projectile/BP_Projectile.BP_Projectile_C" (`KismetMathLibrary.MakeTransform` _returnvalue_location _returnvalue_rotation (0.75 0.75 0.75)) "Undefined" "MultiplyWithRoot" self null))

(event `ActivateInput`
  ;[1 1 1] Initialise controls for the player
  (if (not (`self.bAI`))
    (bind _asbp_first_person_player_controller (cast `/Game/FirstPerson/Blueprints/BP_FirstPersonPlayerController` (`self.GetOwner`)))
    (`/Engine/EditorBlueprintResources/StandardMacros.IsValid` _asbp_first_person_player_controller
      (:`Is Valid`
        (bind _returnvalue (pcsubsystem `EnhancedInputLocalPlayerSubsystem` _asbp_first_person_player_controller))
        (`/Engine/EditorBlueprintResources/StandardMacros.IsValid` _returnvalue
          (:`Is Valid`
            (`EnhancedInputSubsystemInterface.AddMappingContext` _returnvalue "/Game/FirstPerson/Input/IMC_Default.IMC_Default" 0 (struct))
            (`self.EnableInput` null))))
      (:`Is Not Valid`
        (`KismetSystemLibrary.PrintString` "Failed controller cast")))))

(event `EnhancedInput|/Game/FirstPerson/Input/Actions/IA_Look`
  (params (ActionValue :type "Vector2D Structure") (ElapsedSeconds :type "Float (double-precision)") (TriggeredSeconds :type "Float (double-precision)") (InputAction :type "InputAction Object Reference" :default "/Game/FirstPerson/Input/Actions/IA_Look.IA_Look"))
  ;[1 1 1] Look aroud left and right
  (:`Triggered`
    (`self.AddControllerYawInput` ActionValue_X)))

(event `EnhancedInput|/Game/FirstPerson/Input/Actions/IA_Pause`
  (params (ActionValue :type Boolean) (ElapsedSeconds :type "Float (double-precision)") (TriggeredSeconds :type "Float (double-precision)") (InputAction :type "InputAction Object Reference" :default "/Game/FirstPerson/Input/Actions/IA_Pause.IA_Pause"))
  (bind _refgameinst (`self.RefGameInst`))
  (bind _refpausewidget (`self.RefPauseWidget`))
  ;[1 1 1] Pause game
  (:`Started`
    (`Widget.SetVisibility` _refpausewidget "Visible")
    (`BZGameInstance.MenuInputMode` _refgameinst)
    (bind _returnvalue (`GameplayStatics.GetCurrentLevelName` true))
    (if (`KismetStringLibrary.EqualEqual_StrStr` _returnvalue "SoloLevel")
      (`GameplayStatics.SetGamePaused` true)))
  (:`Completed`
    (`Widget.SetVisibility` _refpausewidget "Hidden")
    (`BZGameInstance.GameplayInputMode` _refgameinst)
    (bind _returnvalue_2 (`GameplayStatics.GetCurrentLevelName` true))
    (if true
      (`GameplayStatics.SetGamePaused` false))))

(event `EnhancedInput|/Game/FirstPerson/Input/Actions/IA_Move`
  (params (ActionValue :type "Vector2D Structure") (ElapsedSeconds :type "Float (double-precision)") (TriggeredSeconds :type "Float (double-precision)") (InputAction :type "InputAction Object Reference" :default "/Game/FirstPerson/Input/Actions/IA_Move.IA_Move"))
  (bind (_returnvalue_roll _returnvalue_pitch _returnvalue_yaw) (`KismetMathLibrary.BreakRotator` (`self.GetControlRotation`)))
  (bind (_returnvalue_roll_2 _returnvalue_pitch_2 _returnvalue_yaw_2) (`KismetMathLibrary.BreakRotator` (`self.GetControlRotation`)))
  ;[1 1 1] Move around
  (:`Triggered`
    (if (`self.bAlive`)
      (`self.AddMovementInput` (`KismetMathLibrary.GetRightVector` (`KismetMathLibrary.MakeRotator` _returnvalue_roll_2 0.0 _returnvalue_yaw_2)) ActionValue_X)
      (`self.AddMovementInput` (`KismetMathLibrary.GetForwardVector` (`KismetMathLibrary.MakeRotator` 0.0 0.0 _returnvalue_yaw)) ActionValue_Y))))

(event `EnhancedInput|/Game/FirstPerson/Input/Actions/IA_Shoot`
  (params (ActionValue :type Boolean) (ElapsedSeconds :type "Float (double-precision)") (TriggeredSeconds :type "Float (double-precision)") (InputAction :type "InputAction Object Reference" :default "/Game/FirstPerson/Input/Actions/IA_Shoot.IA_Shoot"))
  ;[1 1 1] Shooting
  (:`Triggered`
    (if (and (`self.bCanShoot`) (`self.bAlive`))
      (set `self.bCanShoot` false)
      (`self.Shooting`)
      (`KismetSystemLibrary.Delay` (`self.FireRate`))
      (set `self.bCanShoot` true))))

(event `self.CollisionBox.OnComponentBeginOverlap`
  (params (OverlappedComponent :type "PrimitiveComponent Object Reference") (OtherActor :type "Actor Object Reference") (OtherComp :type "PrimitiveComponent Object Reference") (OtherBodyIndex :type Integer) (bFromSweep :type Boolean) (SweepResult :type "HitResult Structure (by ref)"))
  ;[1 1 1] The tank got hit. Different outcome if the tank has the powerup or not:
  (if (`self.bAlive`)
    (bind _asbzprojectile (cast `BZProjectile` OtherActor))
    (`/Engine/EditorBlueprintResources/StandardMacros.IsValid` _asbzprojectile
      (:`Is Valid`
        (if (not (== (`self.GetOwner` _asbzprojectile) self))
          (if (`self.bHasPower`)
            ;[1 1 1] Consume power up
            (bind _output_get (set `self.bHasPower` false))
            (`SceneComponent.SetVisibility` (`self.PowerUpShield`) _output_get false)
            (`/Game/Battlezone/CoreBlueprints/BP_BZPlayerState.HasPower` (`self.RefPlayerState`) false)
            (`self.K2_DestroyActor` _asbzprojectile)
            (else
              ;[1 1 1] The tank has been destroyed, initiate the logic to award points and respawn
              (set `self.bAlive` false)
              (`self.TankDisabled`)
              (bind _returnvalue (`self.GetOwner` _asbzprojectile))
              (bind _asbp_tank_player (cast `/Game/Battlezone/Tank/BP_TankPlayer` _returnvalue)
                (:`then`
                  ;[1 1 1] If it PVP, give the kill to the perpetrator
                  (`/Engine/EditorBlueprintResources/StandardMacros.IsValid` _asbp_tank_player
                    (:`Is Valid`
                      (bind _returnvalue_2 (`self.GetController` _asbp_tank_player))
                      (`/Engine/EditorBlueprintResources/StandardMacros.IsValid` _returnvalue_2
                        (:`Is Valid`
                          (bind _asbp_bzplayer_state (cast `/Game/Battlezone/CoreBlueprints/BP_BZPlayerState` (`Controller.PlayerState` _returnvalue_2)))
                          (`self.DestroyedTank` _asbp_bzplayer_state)
                          (`self.K2_DestroyActor` _asbzprojectile))
                        (:`Is Not Valid`
                          (`KismetSystemLibrary.PrintString` "Can't get ennemy Controller"))))))
                (:`CastFailed`
                  ;[1 1 1] PVE
                  (cast `/Game/Battlezone/Tank/BP_TankAI` _returnvalue)
                  (bind _asbp_bzplayer_state_2 (cast `/Game/Battlezone/CoreBlueprints/BP_BZPlayerState` (`self.PlayerState`)))
                  (`/Engine/EditorBlueprintResources/StandardMacros.IsValid` _asbp_bzplayer_state_2
                    (:`Is Valid`
                      (`/Game/Battlezone/CoreBlueprints/BP_SoloGameState.PlayerKilled` (`self.RefPVEGameState`) _asbp_bzplayer_state_2)
                      (`self.K2_DestroyActor` _asbzprojectile :!label _label)
                      (`KismetSystemLibrary.Delay` 3.25)
                      (`self.K2_DestroyActor`)
                      (goto _label))))))))))))

(event `DestroyedTank`
  (params (ScoringPlayer :type "/Game/Battlezone/CoreBlueprints/BP_BZPlayerState Object Reference"))
  ;[1 1 1] Call the GameState to run the logic to award points/revive the player (after letting him chill for 5 seconds of death)
  (`KismetSystemLibrary.Delay` 5.0)
  (bind _asbp_bzplayer_state (cast `/Game/Battlezone/CoreBlueprints/BP_BZPlayerState` (`Controller.PlayerState` (`self.GetController`))))
  (`/Engine/EditorBlueprintResources/StandardMacros.IsValid` _asbp_bzplayer_state
    (:`Is Valid`
      (`/Game/Battlezone/CoreBlueprints/BP_BZGameState.PlayerDestroyed` (`self.PVPGameState`) ScoringPlayer _asbp_bzplayer_state))))

(event `PickedPowerUp`
  (params (PowerUp :type "/Game/Battlezone/PowerUp/BP_PowerUp Object Reference"))
  ;[1 1 1] Pick up PowerUp and consum it's pickable (if the tank doesn't have the power up)
  (if (not (`self.bHasPower`))
    (bind _output_get (set `self.bHasPower` true))
    (`SceneComponent.SetVisibility` (`self.PowerUpShield`) _output_get false)
    (`/Game/Battlezone/PowerUp/BP_PowerUp.ConsumePickable` PowerUp)
    (`/Game/Battlezone/CoreBlueprints/BP_BZPlayerState.HasPower` (`self.RefPlayerState`) true)))

(event `self.ReceiveUnpossessed`
  (params (OldController :type "Controller Object Reference"))
  ;[1 1 1] When unpossessed, Destroy this actor
  (`self.K2_DestroyActor`))

(event `self.ReceiveTick`
  (params (DeltaSeconds :type "Float (single-precision)"))
  (bind _returnvalue (`self.K2_GetActorLocation`))
  ;[1 1 1] Distance from player to enemy
  (bind (_outhit _returnvalue_2) (`KismetSystemLibrary.LineTraceSingleForObjects` _returnvalue (+ (* (`KismetMathLibrary.GetForwardVector` (`self.K2_GetActorRotation`)) (100000.0 100000.0 100000.0)) _returnvalue) (`self.Object Types`)))
  (if _returnvalue_2
    (bind (_bblockinghit _binitialoverlap _time _distance _location _impactpoint _normal _impactnormal _physmat _hitactor) (`GameplayStatics.BreakHitResult` _outhit))
    (bind _asbp_tank_player (cast `/Game/Battlezone/Tank/BP_TankPlayer` _hitactor)
      (:`then`
        (`/Engine/EditorBlueprintResources/StandardMacros.IsValid` _asbp_tank_player
          (:`Is Valid`
            _)
          (:`Is Not Valid`
            (bind _asbp_tank_ai (cast `/Game/Battlezone/Tank/BP_TankAI` _hitactor :!label _label_2))
            (`/Engine/EditorBlueprintResources/StandardMacros.IsValid` _asbp_tank_ai
              (:`Is Valid`
                _)))))
      (:`CastFailed`
        (goto _label_2)))
    (`/Game/Battlezone/CoreBlueprints/BP_BZPlayerState.Distance to enemy` (`self.RefPlayerState`) _distance)
    (else
      (`/Game/Battlezone/CoreBlueprints/BP_BZPlayerState.Distance to enemy` (`self.RefPlayerState`) 0.0))))

(fn `UserConstructionScript`
  (`SceneComponent.SetVisibility` (`self.PowerUpShield`) false false))