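; BP_TankAI is the AI-controlled bot tank in Battlezone, handling hits, power-up pickup and player sighting.
; An overlapping projectile from another owner either consumes the shield power-up or destroys the tank, reporting the kill to BP_SoloGameState.
; Pickups grant the shield only when none is held.
; Sight perception writes the player to the blackboard's TargetActor, clearing it when sight fails or another actor is perceived.
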(event `self.ReceiveBeginPlay`
  ;[1 1 1] Initialise game state ref
  (bind _asbp_solo_game_state (cast `/Game/Battlezone/CoreBlueprints/BP_SoloGameState` (`GameplayStatics.GetGameState`)))
  (`/Engine/EditorBlueprintResources/StandardMacros.IsValid` _asbp_solo_game_state
    (:`Is Valid`
      (set `self.RefGameState` _asbp_solo_game_state)
      ;[1 1 1] Initialise Game instant ref
      (bind _asbzgame_instance (cast `BZGameInstance` (`GameplayStatics.GetGameInstance`)))
      (`/Engine/EditorBlueprintResources/StandardMacros.IsValid` _asbzgame_instance
        (:`Is Valid`
          (set `self.RefGameInst` _asbzgame_instance)
          ;[1 1 1] Starting values
          (set `self.bHasPower` false)
          (set `self.bCanShoot` true)
          ;[1 1 1] Blackboard ref
          (set `self.RefBlackboard` (`AIBlueprintHelperLibrary.GetBlackboard` (`AIBlueprintHelperLibrary.GetAIController` self))))))))

(event `self.CollisionBox.OnComponentBeginOverlap`
  (params (OverlappedComponent :type "PrimitiveComponent Object Reference") (OtherActor :type "Actor Object Reference") (OtherComp :type "PrimitiveComponent Object Reference") (OtherBodyIndex :type Integer) (bFromSweep :type Boolean) (SweepResult :type "HitResult Structure (by ref)"))
  ;[1 1 1] The tank got hit. Different outcome if the tank has the powerup or not:
  (bind _asbzprojectile (cast `BZProjectile` OtherActor))
  (`/Engine/EditorBlueprintResources/StandardMacros.IsValid` _asbzprojectile
    (:`Is Valid`
      (bind _returnvalue (`self.GetOwner` _asbzprojectile))
      (if (not (== _returnvalue self))
        (if (`self.bHasPower`)
          ;[1 1 1] Consume power up
          (bind _output_get (set `self.bHasPower` false))
          (`SceneComponent.SetVisibility` (`self.PowerUpShield`) _output_get false)
          (`self.K2_DestroyActor` _asbzprojectile)
          (else
            ;[1 1 1] The tank has been destroyed, initiate the logic to award points and respawn
            (`/Game/Battlezone/CoreBlueprints/BP_SoloGameState.BotKilled` (`self.RefGameState`) _returnvalue)
            (`self.K2_DestroyActor` _asbzprojectile)
            (`self.K2_DestroyActor`)))))))

(event `PickedPowerUp`
  (params (PowerUp :type "/Game/Battlezone/PowerUp/BP_PowerUp Object Reference"))
  ;[1 1 1] Pick up PowerUp and consum it's pickable (if the tank doesn't have the power up)
  (if (not (`self.bHasPower`))
    (bind _output_get (set `self.bHasPower` true))
    (`SceneComponent.SetVisibility` (`self.PowerUpShield`) _output_get false)
    (`/Game/Battlezone/PowerUp/BP_PowerUp.ConsumePickable` PowerUp)))

(event `self.AIPerception.OnTargetPerceptionUpdated`
  (params (Actor :type "Actor Object Reference") (Stimulus :type "AIStimulus Structure"))
  ;[1 1 1] AI perception (sight)
  (`self.HandleSightSense` Actor Stimulus))

(fn `HandleSightSense`
  (params (Actor :type "Actor Object Reference") (Stimulus :type "AIStimulus Structure"))
  (bind (_stimulus_age _stimulus_expirationage _stimulus_strength _stimulus_stimuluslocation _stimulus_receiverlocation _stimulus_tag _stimulus_bsuccessfullysensed) (break `AIStimulus` (`local.Stimulus`)))
  ;[1 1 1] Make sure we detected something through sight
  (bind _returnvalue (`AIPerceptionSystem.GetSenseClassForStimulus` Stimulus))
  (if (== _returnvalue "/Script/AIModule.AISense_Sight")
    ;[1 1 1] If the detected actor is the player:
    (bind _asbp_tank_player (cast `/Game/Battlezone/Tank/BP_TankPlayer` (`local.Actor`))
      (:`then`
        ;[1 1 1] Set the player as a blackboard variable. If the bot failed to "see" him, then see the player variable to null
        (`BlackboardComponent.SetValueAsObject` (`self.RefBlackboard`) "TargetActor" (`KismetMathLibrary.SelectObject` _asbp_tank_player null _stimulus_bsuccessfullysensed))
        (return))
      (:`CastFailed`
        ;[1 1 1] Set the player variable to null
        (`BlackboardComponent.SetValueAsObject` (`self.RefBlackboard`) "TargetActor" null)
        (return)))
    (else
      (return))))

(fn `UserConstructionScript`
  (`SceneComponent.SetVisibility` (`self.PowerUpShield`) false false))