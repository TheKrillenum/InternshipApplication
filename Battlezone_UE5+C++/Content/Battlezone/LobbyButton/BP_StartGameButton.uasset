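; BP_StartGameButton is a Battlezone lobby trigger actor that starts the match when a first-person player walks into it.
; On BeginPlay it caches the BP_BZGameMode.
; When a BP_FirstPersonCharacter begins overlapping its Box component, it calls TravelToMatch on that game mode.
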(event `self.ReceiveBeginPlay`
  (bind _asbp_bzgame_mode (cast `/Game/Battlezone/CoreBlueprints/BP_BZGameMode` (`GameplayStatics.GetGameMode`)))
  (`/Engine/EditorBlueprintResources/StandardMacros.IsValid` _asbp_bzgame_mode
    (:`Is Valid`
      (set `self.RefGameMode` _asbp_bzgame_mode))))

(event `self.Box.OnComponentBeginOverlap`
  (params (OverlappedComponent :type "PrimitiveComponent Object Reference") (OtherActor :type "Actor Object Reference") (OtherComp :type "PrimitiveComponent Object Reference") (OtherBodyIndex :type Integer) (bFromSweep :type Boolean) (SweepResult :type "HitResult Structure (by ref)"))
  (bind _refgamemode (`self.RefGameMode`))
  (bind _asbp_first_person_character (cast `/Game/FirstPerson/Blueprints/BP_FirstPersonCharacter` OtherActor))
  (`/Engine/EditorBlueprintResources/StandardMacros.IsValid` _asbp_first_person_character
    (:`Is Valid`
      (if (`KismetSystemLibrary.IsValid` _refgamemode)
        (`/Game/Battlezone/CoreBlueprints/BP_BZGameMode.TravelToMatch` _refgamemode)))))

(fn `UserConstructionScript`)