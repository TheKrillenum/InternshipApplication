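; Enemy AI character that patrols between two locations and serves as a target for the lava and crystal guns, reappearing with full HP after death.
; Lava hits swap materials, stack a slow and start a recursive countdown that deals damage each second.
; Crystal hits fill a meter whose milestones deal damage and build to a burst; Tick drains it once released.
; Tick also turns HP and countdown texts toward the player.
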(event `self.ReceiveBeginPlay`
  ;[1 1 1] Initialise variables and starts AI back and forth
  (`self.Back&Forth`)
  (set `self.DefaultSpeed` (`CharacterMovementComponent.MaxWalkSpeed` (`self.CharacterMovement`)))
  (set `self.DefaultMaterial1` (`PrimitiveComponent.GetMaterial` (`self.Mesh`) 0))
  (set `self.DefaultMaterial2` (`PrimitiveComponent.GetMaterial` (`self.Mesh`) 1))
  (`SceneComponent.SetVisibility` (`self.Seconds`) false false)
  (bind _returnvalue (`GameplayStatics.GetActorOfClass` "/Game/FirstPerson/Blueprints/BP_FirstPersonCharacter.BP_FirstPersonCharacter_C"))
  (set `self.Player` _returnvalue))

(event `Back&Forth`
  ;[1 1 1] Moves the Ai back and forth two positions
  (`|AIMoveTo` self (`self.Location1`) null 5.0 true
    (:`OnSuccess`
      (`KismetSystemLibrary.Delay` 1.5)
      (`|AIMoveTo` self (`self.Location2`) null 5.0 true
        (:`OnSuccess`
          (`KismetSystemLibrary.Delay` 1.5)
          (`self.Back&Forth`))))))

(event `LavaGunHit`
  (params (LavaPuddle :type Boolean))
  (bind _mesh (`self.Mesh`))
  (bind _charactermovement (`self.CharacterMovement`))
  (bind _charactermovement_2 (`self.CharacterMovement`))
  (bind _maxwalkspeed (`CharacterMovementComponent.MaxWalkSpeed` (`self.CharacterMovement`)))
  (bind _returnvalue (`KismetStringLibrary.Conv_DoubleToString` _maxwalkspeed))
  (bind _returnvalue_2 (/ (* _maxwalkspeed 100.0) (`self.DefaultSpeed`)))
  ;[1 1 1] Logic applied when a lava bullet hits this character
  (`|ExecutionSequence`
    (:`then_0`
      (`PrimitiveComponent.SetMaterial` _mesh 0 "/Game/Lava_Mat.Lava_Mat")
      (`PrimitiveComponent.SetMaterial` _mesh 1 "/Game/Lava_Mat.Lava_Mat")
      (if LavaPuddle
        ;[1 1 1] Puddle hit logic
        (set `CharacterMovementComponent.MaxWalkSpeed` (* (`self.DefaultSpeed`) 0.4) _charactermovement_2)
        (set `self.Timer` 5)
        (`self.LavaGunTimer` :!label _label)
        (`SceneComponent.SetVisibility` (`self.Seconds`) true false)
        (elif (== (`self.Timer`) 0)
          (set `CharacterMovementComponent.MaxWalkSpeed` (* (`CharacterMovementComponent.MaxWalkSpeed` _charactermovement_2) 0.7) _charactermovement_2)
          (set `self.Timer` 5)
          (goto _label)
          (else
            (if (not (== (`CharacterMovementComponent.MaxWalkSpeed` (`self.CharacterMovement`)) (* (`self.DefaultSpeed`) 0.4)))
              (set `CharacterMovementComponent.MaxWalkSpeed` (- (`CharacterMovementComponent.MaxWalkSpeed` _charactermovement) (* (`self.DefaultSpeed`) 0.1)) _charactermovement))
            (set `self.Timer` 5)))))
    (:`then_1`
      (if (== _returnvalue_2 60.0)
        (`KismetSystemLibrary.PrintString` (`KismetStringLibrary.Concat_StrStr` "60% MAX SLOW (speed at" (`KismetStringLibrary.Concat_StrStr` _returnvalue ")")))
        (else
          (`KismetSystemLibrary.PrintString` (`KismetStringLibrary.Concat_StrStr` (`KismetStringLibrary.Conv_DoubleToString` _returnvalue_2) (`KismetStringLibrary.Concat_StrStr` "% slow (speed at " (`KismetStringLibrary.Concat_StrStr` _returnvalue ")")))))))))

(event `LavaGunTimer`
  (bind _mesh (`self.Mesh`))
  ;[1 1 1] Timer for the duration of the lava slow
  (bind _result (`/Engine/EditorBlueprintResources/StandardMacros.DecrementInt` (`self.Timer`))
    (:`  `
      (`TextRenderComponent.K2_SetText` (`self.Seconds`) (`KismetTextLibrary.Conv_IntToText` _result))
      (if (<= _result 0)
        (set `self.Timer` 0)
        (`PrimitiveComponent.SetMaterial` _mesh 0 (`self.DefaultMaterial1`))
        (`PrimitiveComponent.SetMaterial` _mesh 1 (`self.DefaultMaterial2`))
        (bind _output_get (set `CharacterMovementComponent.MaxWalkSpeed` (`self.DefaultSpeed`) (`self.CharacterMovement`)))
        (`KismetSystemLibrary.PrintString` (`KismetStringLibrary.Concat_StrStr` "0% slow (speed at " (`KismetStringLibrary.Concat_StrStr` (`KismetStringLibrary.Conv_DoubleToString` _output_get) ")")))
        (`SceneComponent.SetVisibility` (`self.Seconds`) false false)
        (else
          (`self.TakingDamages` 5.0)
          (`KismetSystemLibrary.Delay` 1.0)
          (`self.LavaGunTimer`))))))

(event `TakingDamages`
  (params (Damage :type "Float (double-precision)"))
  ;[1 1 1] Damage logic (and death)
  (bind _output_get (set `self.HP` (- (`self.HP`) Damage)))
  (if (<= _output_get 0.0)
    (`self.Death`)))

(event `self.ReceiveAnyDamage`
  (params (Damage :type "Float (single-precision)") (DamageType :type "DamageType Object Reference") (InstigatedBy :type "Controller Object Reference") (DamageCauser :type "Actor Object Reference"))
  ;[1 1 1] Delegate damage to damage logic
  (`self.TakingDamages` Damage))

(event `self.ReceiveTick`
  (params (DeltaSeconds :type "Float (single-precision)"))
  (bind _healthpoints (`self.HealthPoints`))
  (bind _player (`self.Player`))
  (bind _seconds (`self.Seconds`))
  ;[1 1 1] Adjust the display rotation and update health
  (`TextRenderComponent.K2_SetText` _healthpoints (`KismetTextLibrary.Conv_DoubleToText` (`self.HP`) "HalfToEven"))
  (`SceneComponent.K2_SetWorldRotation` _healthpoints (`KismetMathLibrary.FindLookAtRotation` (`SceneComponent.K2_GetComponentLocation` _healthpoints) (`self.K2_GetActorLocation` _player)) false false)
  (`SceneComponent.K2_SetWorldRotation` _seconds (`KismetMathLibrary.FindLookAtRotation` (`SceneComponent.K2_GetComponentLocation` _seconds) (`self.K2_GetActorLocation` _player)) false false)
  ;[1 1 1] Empty the crystal gun's meter
  (if (`self.CrystalReduce`)
    (bind _result (`/Engine/EditorBlueprintResources/StandardMacros.DecrementFloat` (`self.CrystalMeter`))
      (:`  `
        (if (and (<= _result 0.0) (>= (`self.CrystalMilestone`) 1.0))
          (`/Engine/EditorBlueprintResources/StandardMacros.DecrementFloat` (`self.CrystalMilestone`)
            (:`  `
              (set `self.CrystalMeter` 25.0)))
          (elif (and (<= (`self.CrystalMeter`) 0.0) (<= (`self.CrystalMilestone`) 0.0))
            (set `self.CrystalReduce` false)))))))

(event `Death`
  ;[1 1 1] Death timer
  (`SceneComponent.SetVisibility` (`self.CapsuleComponent`) false true)
  (`KismetSystemLibrary.Delay` 2.0)
  (set `self.HP` 100.0)
  (`SceneComponent.SetVisibility` (`self.CapsuleComponent`) true true))

(event `CrystalDamage`
  (params (DeltaTime :type "Float (double-precision)"))
  (bind _crystalmeter (`self.CrystalMeter`))
  ;[1 1 1] Crystal gun damage logic and meter fill up
  (set `self.CrystalReduce` false)
  (`/Engine/EditorBlueprintResources/StandardMacros.IncrementFloat` _crystalmeter
    (:`  `
      (if (>= _crystalmeter 25.0)
        (set `self.CrystalMeter` 0.0)
        (`self.TakingDamages` 5.0)
        (bind _result (`/Engine/EditorBlueprintResources/StandardMacros.IncrementFloat` (`self.CrystalMilestone`))
          (:`  `
            (if (>= _result 6.0)
              (set `self.CrystalMilestone` 0.0)
              (`self.TakingDamages` 70.0))))))))

(event `ResetMeter`
  ;[1 1 1] Crystal gun meter emptying
  (set `self.CrystalReduce` true))

(fn `UserConstructionScript`)