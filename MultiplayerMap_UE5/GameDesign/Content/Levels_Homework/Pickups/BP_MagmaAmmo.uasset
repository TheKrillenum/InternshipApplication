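; BP_MagmaAmmo is a pickup that grants the player lava ammo.
; It overrides PickupEffect, calling the parent effect, adding a fixed amount to the player's LavaAmmo, then passing the new total to UpdateLavaAmmo.
; The event graph holds only disabled stubs and the construction script just calls its parent, so all other behavior is inherited from the parent class.
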(fn `PickupEffect`
  (params (Player :type "/Game/FirstPerson/Blueprints/BP_FirstPersonCharacter Object Reference"))
  (`parent.PickupEffect` Player)
  (bind _output_get (set `/Game/FirstPerson/Blueprints/BP_FirstPersonCharacter.LavaAmmo` (+ (`/Game/FirstPerson/Blueprints/BP_FirstPersonCharacter.LavaAmmo` Player) 6) Player))
  (`/Game/FirstPerson/Blueprints/BP_FirstPersonCharacter.UpdateLavaAmmo` Player _output_get)
  (return))

(fn `UserConstructionScript`
  (`parent.UserConstructionScript`))