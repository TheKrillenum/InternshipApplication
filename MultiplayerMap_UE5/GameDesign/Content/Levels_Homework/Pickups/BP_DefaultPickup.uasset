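; BP_DefaultPickup is a base pickup that a BP_FirstPersonCharacter collects by overlapping its Sphere.
; On pickup it goes inactive, hides its Cube and calls PickupEffect with the player, then reappears and reactivates after a fixed five-second delay.
; PickupEffect is an empty function here, serving as a hook for a specific effect.
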(event `self.ReceiveActorBeginOverlap`
  (params (OtherActor :type "Actor Object Reference")))

(event `self.Sphere.OnComponentBeginOverlap`
  (params (OverlappedComponent :type "PrimitiveComponent Object Reference") (OtherActor :type "Actor Object Reference") (OtherComp :type "PrimitiveComponent Object Reference") (OtherBodyIndex :type Integer) (bFromSweep :type Boolean) (SweepResult :type "HitResult Structure (by ref)"))
  (if (`self.Active`)
    (bind _asbp_first_person_character (cast `/Game/FirstPerson/Blueprints/BP_FirstPersonCharacter` OtherActor))
    (set `self.Active` false)
    (`SceneComponent.SetVisibility` (`self.Cube`) false true)
    (`self.PickupEffect` _asbp_first_person_character)
    (`KismetSystemLibrary.Delay` 5.0)
    (`SceneComponent.SetVisibility` (`self.Cube`) true true)
    (set `self.Active` true)))

(fn `PickupEffect`
  (params (Player :type "/Game/FirstPerson/Blueprints/BP_FirstPersonCharacter Object Reference"))
  (return))

(fn `UserConstructionScript`)