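; BP_DefaultGimmick is a level gimmick whose Cube component endlessly moves up and back down.
; On BeginPlay it stores the Cube's relative location, eases it up on Z by MoveDistance with MoveComponentTo, pauses, then eases it back to the stored spot.
; After a second pause, a custom Repeat event loops back to the upward move.
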(event `self.ReceiveBeginPlay`
  (bind _returnvalue (`SceneComponent.GetRelativeTransform` (`self.Cube`)))
  (bind _returnvalue_location (`KismetMathLibrary.BreakTransform` (`SceneComponent.GetRelativeTransform` (`self.Cube`))))
  ;[1 1 1] Start the script, and saves the original actor location
  (set `self.OriginalActorLocation` _returnvalue_location)
  ;[1 1 1] Slowly move component up
  (`KismetSystemLibrary.MoveComponentTo` (`self.Cube`) (`KismetMathLibrary.MakeVector` (.x (.location _returnvalue)) (.y (.location _returnvalue)) (+ (.z (.location _returnvalue)) (`self.MoveDistance`))) (struct) true true 3.0 :!label _label)
  ;[1 1 1] Wait 3 seconds
  (`KismetSystemLibrary.Delay` 3.0)
  ;[1 1 1] Slowly move component back to it's original location
  (`KismetSystemLibrary.MoveComponentTo` (`self.Cube`) (`self.OriginalActorLocation`) (struct) true true 3.0)
  ;[1 1 1] Wait 3 seconds
  (`KismetSystemLibrary.Delay` 3.0)
  ;[1 1 1] Repeat the whole process
  (`self.Repeat`))

(event `Repeat`
  (goto _label))

(fn `UserConstructionScript`)