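; BP_GimmckCross is a level gimmick whose GimmickCross component endlessly rises and returns to its starting position.
; BeginPlay stores the component's relative location, then waits a per-instance DelayBetweenPillars so that placed copies can be staggered.
; Eased MoveComponentTo calls raise it by MoveDistance and bring it back, pausing after each move.
; A Repeat event loops back to the upward move, skipping the initial delay.
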(event `self.ReceiveBeginPlay`
  (bind _gimmick_cross (`self.Gimmick_Cross`))
  (bind _gimmick_cross_2 (`self.Gimmick_Cross`))
  (bind _returnvalue (`SceneComponent.GetRelativeTransform` _gimmick_cross_2))
  (bind _returnvalue_location (`KismetMathLibrary.BreakTransform` (`SceneComponent.GetRelativeTransform` (`self.Gimmick_Cross`))))
  ;[1 1 1] Start the script, and saves the original actor location
  (set `self.OriginalActorLocation` _returnvalue_location)
  ;[1 1 1] Enable delay at the start which can modified per instance
  (`KismetSystemLibrary.Delay` (`self.DelayBetweenPillars`))
  ;[1 1 1] Slowly move component up
  (`KismetSystemLibrary.MoveComponentTo` _gimmick_cross_2 (`KismetMathLibrary.MakeVector` (.x (.location _returnvalue)) (.y (.location _returnvalue)) (+ (.z (.location _returnvalue)) (`self.MoveDistance`))) (.rotation _returnvalue) true true 3.0 :!label _label)
  ;[1 1 1] Wait 3 seconds
  (`KismetSystemLibrary.Delay` 3.0)
  ;[1 1 1] Slowly move component back to it's original location
  (`KismetSystemLibrary.MoveComponentTo` _gimmick_cross (`self.OriginalActorLocation`) (`SceneComponent.RelativeRotation` _gimmick_cross) true true 3.0)
  ;[1 1 1] Wait 3 seconds
  (`KismetSystemLibrary.Delay` 3.0)
  ;[1 1 1] Repeat the whole process
  (`self.Repeat`))

(event `Repeat`
  ;[1 1 1] Slowly move component up
  (goto _label))

(fn `UserConstructionScript`)