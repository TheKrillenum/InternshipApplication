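; Gimmick elevator actor that endlessly moves its ElevatorSmallRoom component up and back down.
; BeginPlay saves the room's starting relative location, then waits a per-instance DelayBetweenPillars before the first move.
; Eased MoveComponentTo calls raise it by MoveDistance and return it, pausing after each move.
; A Repeat custom event restarts the cycle without repeating the initial delay.
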(event `self.ReceiveBeginPlay`
  (bind _elevator_smallroom (`self.Elevator_smallRoom`))
  (bind _elevator_smallroom_2 (`self.Elevator_smallRoom`))
  (bind _returnvalue (`SceneComponent.GetRelativeTransform` _elevator_smallroom_2))
  (bind _returnvalue_location (`KismetMathLibrary.BreakTransform` (`SceneComponent.GetRelativeTransform` (`self.Elevator_smallRoom`))))
  ;[1 1 1] Start the script, and saves the original actor location
  (set `self.OriginalActorLocation` _returnvalue_location)
  ;[1 1 1] Enable delay at the start which can modified per instance
  (`KismetSystemLibrary.Delay` (`self.DelayBetweenPillars`))
  ;[1 1 1] Slowly move component up
  (`KismetSystemLibrary.MoveComponentTo` _elevator_smallroom_2 (`KismetMathLibrary.MakeVector` (.x (.location _returnvalue)) (.y (.location _returnvalue)) (+ (.z (.location _returnvalue)) (`self.MoveDistance`))) (.rotation _returnvalue) true true 3.0 :!label _label)
  ;[1 1 1] Wait 3 seconds
  (`KismetSystemLibrary.Delay` 3.0)
  ;[1 1 1] Slowly move component back to it's original location
  (`KismetSystemLibrary.MoveComponentTo` _elevator_smallroom (`self.OriginalActorLocation`) (`SceneComponent.RelativeRotation` _elevator_smallroom) true true 3.0)
  ;[1 1 1] Wait 3 seconds
  (`KismetSystemLibrary.Delay` 3.0)
  ;[1 1 1] Repeat the whole process
  (`self.Repeat`))

(event `Repeat`
  ;[1 1 1] Slowly move component up
  (goto _label))

(fn `UserConstructionScript`)